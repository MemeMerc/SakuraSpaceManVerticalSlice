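; JumpPad_BP is a platforming jump pad that launches the player along the direction of its Arrow component.
; It caches the Player_BP2 character on BeginPlay and reacts when that player's capsule overlaps the Sphere trigger.
; The launch overrides existing velocity using JumpVelocity, and after a short delay the pad deactivates the player's glide.
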(event `self.ReceiveBeginPlay`
  ;[1 1 1] Created By Lucas
  (bind _asplayer_bp2 (cast `/Game/Blueprints/Player/Player_BP2` (`GameplayStatics.GetPlayerCharacter` 0)))
  (set `self.Player` _asplayer_bp2))

(event `self.Sphere.OnComponentBeginOverlap`
  (params (OverlappedComponent :type "PrimitiveComponent Object Reference") (OtherActor :type "Actor Object Reference") (OtherComp :type "PrimitiveComponent Object Reference") (OtherBodyIndex :type Integer) (bFromSweep :type Boolean) (SweepResult :type "HitResult Structure (by ref)"))
  (bind _player (`self.Player`))
  ;[1 1 1] Created By Lucas
  (if (== OtherComp (`Character.CapsuleComponent` _player))
    (`Character.LaunchCharacter` _player (* (`SceneComponent.GetForwardVector` (`self.Arrow`)) (`self.Jump Velocity`)) true true)
    (`KismetSystemLibrary.Delay` 0.3)
    (`Player_CPP.DeactivateGlide` _player)))

(fn `UserConstructionScript`)