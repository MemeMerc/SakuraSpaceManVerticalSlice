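; BoostPad_BP is a platforming boost pad that launches the player along the pad's forward direction.
; On BeginPlay it caches player 0's character as Player_BP.
; When that capsule overlaps the Box, it sets max walk speed and velocity from a bonus added to one of the player's FMaxSpeed entries, then flags IsBoosting.
; The pad never resets these values itself.
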(event `self.ReceiveBeginPlay`
  (bind _asplayer_bp (cast `/Game/Blueprints/Player/Player_BP` (`GameplayStatics.GetPlayerCharacter` 0)))
  (set `self.Player` _asplayer_bp))

(event `self.Box.OnComponentBeginOverlap`
  (params (OverlappedComponent :type "PrimitiveComponent Object Reference") (OtherActor :type "Actor Object Reference") (OtherComp :type "PrimitiveComponent Object Reference") (OtherBodyIndex :type Integer) (bFromSweep :type Boolean) (SweepResult :type "HitResult Structure (by ref)"))
  (bind _player (`self.Player`))
  (bind _charactermovement (`Character.CharacterMovement` _player))
  (bind _returnvalue (+ (`self.Boost Velocity Bonus`) (`|GetArrayItem` (`Player_CPP.fMaxSpeed` _player) 1)))
  (if (== OtherComp (`Character.CapsuleComponent` _player))
    (set `CharacterMovementComponent.MaxWalkSpeed` _returnvalue _charactermovement)
    (set `MovementComponent.Velocity` (* (`self.GetActorForwardVector`) _returnvalue) _charactermovement)
    (set `Player_CPP.bIsBoosting` true _player)))

(fn `UserConstructionScript`)