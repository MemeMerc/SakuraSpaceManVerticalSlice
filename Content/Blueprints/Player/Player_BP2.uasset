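; Player Blueprint that draws the grapple wire while the player reels in toward a grapple point.
; On Tick, it aims a spline mesh at the GrappleLocation_BP widget and stretches its X end by distance times a scale factor.
; Paired DoOnce nodes reset each other, toggling wire visibility only when reeling starts or stops.
; Grapple sphere end-overlap events are forwarded to GrappleOnOverlapEnd, which is defined outside these graphs.
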(event `self.ReceiveBeginPlay`
  (`SceneComponent.SetVisibility` (`self.SplineMesh`) false false))

(event `self.ReceiveTick`
  (params (DeltaSeconds :type "Float (single-precision)"))
  (bind _splinemesh (`self.SplineMesh`))
  (bind _splinemesh_2 (`self.SplineMesh`))
  (bind _returnvalue (`SceneComponent.K2_GetComponentLocation` (`self.SplineMesh`)))
  ;[1 1 1] Grapple Wire
  (if (`self.bIsReelingIn`)
    (bind _returnvalue_2 (`self.ReturnGrapple`))
    (bind _returnvalue_3 (`SceneComponent.K2_GetComponentLocation` (`/Game/Blueprints/GrappleLocation/GrappleLocation_BP.Widget` (cast `/Game/Blueprints/GrappleLocation/GrappleLocation_BP` _returnvalue_2 :!pure true))))
    (`SceneComponent.K2_SetWorldRotation` _splinemesh (`KismetMathLibrary.FindLookAtRotation` _returnvalue _returnvalue_3) false false)
    (`SplineMeshComponent.SetEndPosition` _splinemesh (`KismetMathLibrary.MakeVector` (* (`KismetMathLibrary.Vector_Distance` _returnvalue _returnvalue_3) 4.0)) true)
    (`/Engine/EditorBlueprintResources/StandardMacros.DoOnce` false :!label _label
      (:`Completed`
        (`SceneComponent.SetVisibility` _splinemesh_2 true false)
        (goto _label_2 :!via `Reset`)))
    (else
      (`/Engine/EditorBlueprintResources/StandardMacros.DoOnce` false :!label _label_2
        (:`Completed`
          (`SceneComponent.SetVisibility` _splinemesh_2 false false)
          (goto _label :!via `Reset`))))))

(event `self.GrappleCollisionSphere.OnComponentEndOverlap`
  (params (OverlappedComponent :type "PrimitiveComponent Object Reference") (OtherActor :type "Actor Object Reference") (OtherComp :type "PrimitiveComponent Object Reference") (OtherBodyIndex :type Integer))
  (`self.Grapple_OnOverlapEnd` OverlappedComponent OtherActor OtherComp OtherBodyIndex))

(fn `UserConstructionScript`)